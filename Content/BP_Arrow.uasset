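; BP_Arrow is a stationary shooter that tracks the player and repeatedly fires magic projectiles.
; Each tick it rotates to face the first player pawn using a look-at rotation.
; A looping timer set on BeginPlay triggers ArrowAttack, which spawns a BP_SMagicProjectile at the actor's location and rotation, so each shot aims at the player.
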(event `self.ReceiveTick`
  (params (DeltaSeconds :type "Float (single-precision)"))
  (`self.K2_SetActorRotation` (`KismetMathLibrary.FindLookAtRotation` (`self.K2_GetActorLocation`) (`self.K2_GetActorLocation` (`GameplayStatics.GetPlayerPawn` 0)))))

(event `self.ReceiveBeginPlay`
  (`KismetSystemLibrary.K2_SetTimerDelegate` (delegate `ArrowAttack`) 2.0 true))

(event `ArrowAttack`
  (`|SpawnActorFromClass` "/Game/BP_SMagicProjectile.BP_SMagicProjectile_C" (`KismetMathLibrary.MakeTransform` (`self.K2_GetActorLocation`) (`self.K2_GetActorRotation`)) "Undefined" "MultiplyWithRoot" null null))

(fn `UserConstructionScript`)